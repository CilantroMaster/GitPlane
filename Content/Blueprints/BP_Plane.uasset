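; BP_Plane is a player-controllable plane pawn that constantly flies forward along its facing direction.
; Tick spins the Left and Right propellers in opposite roll directions and feeds the actor's forward vector into movement input.
; Roll and Pitch axis inputs rotate the actor locally at RotateSpeed, scaled by delta time, which steers the flight path.
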(event `self.ReceiveTick`
  (params (DeltaSeconds :type "Float (single-precision)"))
  ;[1 1 1] 왼쪽 프로펠러 회전
  (`SceneComponent.K2_AddLocalRotation` (`self.Left`) (`KismetMathLibrary.MakeRotator` (* (`self.Propeller Rotation Speed`) (`GameplayStatics.GetWorldDeltaSeconds`))) false false)
  ;[1 1 1] 오른쪽 프로펠러 회전
  (`SceneComponent.K2_AddLocalRotation` (`self.Right`) (`KismetMathLibrary.MakeRotator` (* (`self.Propeller Rotation Speed`) (`GameplayStatics.GetWorldDeltaSeconds`) -1.0)) false false)
  ;[1 1 1] 비행기 이동
  (`self.AddMovementInput` (`self.GetActorForwardVector`)))

(event `InputAxis|Roll`
  (params (AxisValue :type "Float (single-precision)"))
  ;[1 1 1] Roll 회전
  (`self.K2_AddActorLocalRotation` (`KismetMathLibrary.MakeRotator` (* (`GameplayStatics.GetWorldDeltaSeconds`) (`self.RotateSpeed`) AxisValue))))

(event `InputAxis|Pitch`
  (params (AxisValue :type "Float (single-precision)"))
  ;[1 1 1] Pitch 회전
  (`self.K2_AddActorLocalRotation` (`KismetMathLibrary.MakeRotator` 0.0 (* (`GameplayStatics.GetWorldDeltaSeconds`) (`self.RotateSpeed`) AxisValue))))

(fn `UserConstructionScript`)